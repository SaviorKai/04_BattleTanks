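; Tank Blueprint that turns player input into driving, aiming the camera, and firing.
; BeginPlay wires the barrel and turret into the aiming component, both tracks into the movement component, and the tank into its health bar widget.
; Driving supports manual per-track throttle or "fly-by-wire" intents through the movement component.
; An azimuth gimbal and spring arm rotate the view, with toggles for vertical inversion and first/third-person cameras.
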(event EventBeginPlay
  (Class|TankAimingComponent|InitialiseAimComponent (Variables|Default|GetTankAiming_Component) (Variables|Default|GetBarrel) (Variables|Default|GetTurret))
  (Class|TankMovementComponent|InitialiseMoveComponent (Variables|Default|GetTankMovement) (Variables|Default|GetLeftTrack) (Variables|Default|GetRightTrack))
  (CallFunction|InitializeHealthBarWidget))

(event Input|ActionEvents|InputActionChangeCamera
  (params (Key :type Key%20Structure))
  ;[0.5333 0.6038 1] Camera Swapping
  (:Released
    (Components|Activation|ToggleActive (Variables|Default|GetCamera_3rdPerson))
    (Components|Activation|ToggleActive (Variables|Default|GetCamera_1stPerson))))

(event Input|ActionEvents|InputActionInvertMouseY
  (params (Key :type Key%20Structure))
  ;[0.5333 0.6038 1] Turn on Invert Camera
  (:Released
    (if (Variables|Default|GetbIsInvertCamera)
      (Variables|Default|SetbIsInvertCamera false)
      (Development|PrintString "Invert Mouse = Off" true false)
      (else
        (Variables|Default|SetbIsInvertCamera true)
        (Development|PrintString "Invert Mouse = On" true false)))))

(event Input|ActionEvents|InputActionTankFire
  (params (Key :type Key%20Structure))
  ;[1 1 1] Fire Input Setup
  (:Pressed
    (Class|TankAimingComponent|Fire (Variables|Default|GetTankAiming_Component))))

(event Input|AxisEvents|InputAxisAimAzimuth
  (params (AxisValue :type Float%20%28single-precision%29))
  ;[1 1 1] Camera Input Controls Binding
  (Transformation|AddLocalRotation (Variables|Default|GetScene%20%28Azimuth%20Gimbal%29) (Math|Rotator|MakeRotator 0.0 0.0 AxisValue) false false))

(event Input|AxisEvents|InputAxisAimElevation
  (params (AxisValue :type Float%20%28single-precision%29))
  ;[1 1 1] Camera Input Controls Binding
  (if (Variables|Default|GetbIsInvertCamera)
    ;;[0.5333 0.6038 1] Invert Camera if Bool is True
    (Transformation|AddLocalRotation (Variables|Default|GetSpringArm) (Math|Rotator|MakeRotator 0.0 (* AxisValue -1.0) 0.0) false false)
    (else
      (Transformation|AddLocalRotation (Variables|Default|GetSpringArm) (Math|Rotator|MakeRotator 0.0 AxisValue 0.0) false false))))

(event Input|AxisEvents|InputAxisLeftThrottle
  (params (AxisValue :type Float%20%28single-precision%29))
  ;[1 1 1] Input Setup (Manual Track Movement)
  (Class|TankTrack|SetThrottle (Variables|Default|GetLeftTrack) AxisValue))

(event Input|AxisEvents|InputAxisRightThrottle
  (params (AxisValue :type Float%20%28single-precision%29))
  ;[1 1 1] Input Setup (Manual Track Movement)
  (Class|TankTrack|SetThrottle (Variables|Default|GetRightTrack) AxisValue))

(event Input|AxisEvents|InputAxisIntendForward
  (params (AxisValue :type Float%20%28single-precision%29))
  ;[1 1 1] Input Setup (Auto "Fly-by-wire" Movement)
  (Class|TankMovementComponent|IntendMoveForward (Variables|Default|GetTankMovement) AxisValue))

(event Input|AxisEvents|InputAxisIntendTurnRight
  (params (AxisValue :type Float%20%28single-precision%29))
  ;[1 1 1] Input Setup (Auto "Fly-by-wire" Movement)
  (Class|TankMovementComponent|IntendTurnRight (Variables|Default|GetTankMovement) AxisValue))

(fn ConstructionScript)

(fn InitializeHealthBarWidget
  ;[1 0.8996 0.4012] The "Cast" doesn't affect the previous step in the chain. What it does here, is convert "UserWidgetObject" to "wbp_HealthBar", a child class of the UserWidgetObject.
  (bind _aswbp_health_bar (Utilities|Casting|CastTowbp_HealthBar (UserInterface|GetUserWidgetObject (Variables|Default|GetWidget_HealthBar))))
  (Variables|/Game/UI/wbp_HealthBar.wbp_HealthBar_C|SetMyTank _aswbp_health_bar self))